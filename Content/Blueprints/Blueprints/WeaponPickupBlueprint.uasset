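; Weapon pickup that overwrites the stats of the collecting actor's gun, with a material showing its rarity.
; On BeginPlay the server calls OnGenerate, defined outside this graph, while clients set the mesh material from Rarity.
; OnPickup copies velocity, damage, magazine size and accuracy to the child-actor GunBlueprint and refills its magazine.
; It then updates a player character's ammo HUD through a client event and destroys itself.
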(event `self.ReceiveBeginPlay`
  (if (`KismetSystemLibrary.IsServer`)
    (`self.OnGenerate`)
    (else
      (`self.FunctionSetColour`))))

(event `self.OnPickup`
  (params (ActorThatPickedUp :type "Actor Object Reference"))
  (bind _returnvalue (`self.GetComponentByClass` ActorThatPickedUp "/Script/Engine.ChildActorComponent"))
  (`/Engine/EditorBlueprintResources/StandardMacros.IsValid` _returnvalue
    (:`Is Valid`
      (bind _asgun_blueprint (cast `/Game/Blueprints/Blueprints/GunBlueprint` (`ChildActorComponent.ChildActor` _returnvalue)))
      (set `/Game/Blueprints/Blueprints/GunBlueprint.MuzzleVelocity` (`self.MuzzleVelocity`) _asgun_blueprint)
      (set `/Game/Blueprints/Blueprints/GunBlueprint.BulletDamage` (`self.BulletDamage`) _asgun_blueprint)
      (bind _output_get (set `/Game/Blueprints/Blueprints/GunBlueprint.MagazineSize` (`self.MagazineSize`) _asgun_blueprint))
      (set `/Game/Blueprints/Blueprints/GunBlueprint.WeaponAccuracy` (`self.WeaponAccuracy`) _asgun_blueprint)
      (bind _output_get_2 (set `/Game/Blueprints/Blueprints/GunBlueprint.RoundsRemainingInMagazine` _output_get _asgun_blueprint))
      (bind _asplayer_character_blueprint (cast `/Game/Blueprints/Blueprints/PlayerCharacterBlueprint` ActorThatPickedUp)
        (:`then`
          (`/Game/Blueprints/Blueprints/PlayerCharacterBlueprint.ClientUpdateAmmoHUDEvent` _asplayer_character_blueprint _output_get_2 _output_get))
        (:`CastFailed`
          _))
      (`self.K2_DestroyActor`))))

(fn `FunctionSetColour`
  (switch `EWeaponPickupRarity` (`self.Rarity`)
    (:`LEGENDARY`
      (`PrimitiveComponent.SetMaterial` (`self.SkeletalMesh`) 0 "/Game/Materials/PickupMaterials/LegendaryMaterial.LegendaryMaterial"))
    (:`MASTER`
      (`PrimitiveComponent.SetMaterial` (`self.SkeletalMesh`) 0 "/Game/Materials/PickupMaterials/MasterMaterial.MasterMaterial"))
    (:`RARE`
      (`PrimitiveComponent.SetMaterial` (`self.SkeletalMesh`) 0 "/Game/Materials/PickupMaterials/RareMaterial.RareMaterial"))
    (:`COMMON`
      (`PrimitiveComponent.SetMaterial` (`self.SkeletalMesh`) 0 "/Game/Materials/PickupMaterials/CommonMaterial.CommonMaterial"))))

(fn `UserConstructionScript`)